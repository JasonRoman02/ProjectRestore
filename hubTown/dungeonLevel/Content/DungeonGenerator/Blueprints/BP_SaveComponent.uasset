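; Save component for the dungeon game that handles saving, loading, profile-named autosaves and toggling the save menu.
; Saves record rooms, generated dungeons, listed actor classes and the player's transform, maps and keys in a per-level entry.
; Loading stores the target slot in a "LoadLevel" save, opens that level, then BeginPlay restores it and clears the slot.
; Rooms and generators restore themselves; other actors are moved, respawned or destroyed to match.
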(event Custom|Open_SaveMenu
  (bind _ui_menu (Variables|Default|GetUI_Menu))
  (bind _returnvalue (Widget|GetOwningPlayer _ui_menu))
  ;[1 1 1] Menu
  (if (UserInterface|Viewport|IsinViewport (Variables|Default|GetUI_Menu))
    (Widget|RemovefromParent _ui_menu)
    (Input|SetInputModeGameOnly _returnvalue)
    (Variables|/Script/Engine.PlayerController|SetbShowMouseCursor _returnvalue false)
    (else
      (UserInterface|Viewport|AddtoViewport _ui_menu 0)
      (Input|SetInputModeUIOnly _returnvalue _ui_menu "DoNotLock")
      (Variables|/Script/Engine.PlayerController|SetbShowMouseCursor _returnvalue true)
      (Widget|SetFocus _ui_menu))))

(event Custom|LoadGame
  (params (SlotName :type String))
  (bind _savegames (Variables|Default|GetSavegames))
  ;[1 1 1] Load
  (Development|PrintString "Loaded")
  (bind _returnvalue (SaveGame|LoadGamefromSlot SlotName))
  (bind _asbp_savegame (Utilities|Casting|CastToBP_Savegame _returnvalue))
  (bind _array_element (Utilities|Array|ForEachLoopwithBreak (Variables|/Game/DungeonGenerator/Savegames/BP_Savegame.BP_Savegame_C|GetSavedLevels _asbp_savegame) :!label _label)
    (:LoopBody
      (if (Utilities|Enum|Equal(Enum) (.LevelName (Utilities|Struct|BreakS_SavedLevel _array_element)) (Variables|/Game/DungeonGenerator/Savegames/BP_Savegame.BP_Savegame_C|GetCurrentLevel _asbp_savegame))
        (Utilities|FlowControl|Sequence
          (:then_0
            (goto _label Break))
          (:then_1
            (CallFunction|LoadRooms (.SavedRooms (Utilities|Struct|BreakS_SavedLevel _array_element)))
            (CallFunction|LoadDungeon (.SavedDungeons (Utilities|Struct|BreakS_SavedLevel _array_element)))
            (CallFunction|LoadActors (.SavedActors (Utilities|Struct|BreakS_SavedLevel _array_element)))
            (CallFunction|LoadPlayer (.SaveMainCharacter (Utilities|Struct|BreakS_SavedLevel _array_element)))
            (Variables|/Game/DungeonGenerator/Savegames/BP_Savegame.BP_Savegame_C|SetSlotToLoad _savegames "None")
            (SaveGame|SaveGametoSlot _savegames "LoadLevel")))))))

(event Custom|Autosave
  ;[1 1 1] Profile Autosaves
  (if (Variables|Default|GetAllowAutosaves)
    (CallFunction|SaveGame (Utilities|String|Append (Variables|Default|GetProfileName) "_Autosave1"))))

(event Custom|Load_Autosave
  (params (ProfileName :type String))
  ;[1 1 1] Profile Autosaves
  (CallFunction|LoadLevel (Utilities|String|Append ProfileName "_Autosave1")))

(event Custom|SaveGame
  (params (SlotName :type String))
  (bind _savegames (Variables|Default|GetSavegames))
  (bind _savedlevels (Variables|/Game/DungeonGenerator/Savegames/BP_Savegame.BP_Savegame_C|GetSavedLevels _savegames))
  ;[1 1 1] Save
  (Development|PrintString "Saved")
  (bind _levelindex (CallFunction|SaveLevel))
  (bind _output_get (Variables|Default|SetLevelIndex _levelindex))
  (Utilities|Array|Clear (.SavedRooms (Utilities|Struct|BreakS_SavedLevel (Utilities|Array|Get(acopy) _savedlevels _output_get))))
  (Utilities|Array|Clear (.SavedDungeons (Utilities|Struct|BreakS_SavedLevel (Utilities|Array|Get(acopy) _savedlevels _output_get))))
  (Utilities|Array|Clear (.SavedActors (Utilities|Struct|BreakS_SavedLevel (Utilities|Array|Get(acopy) _savedlevels _output_get))))
  (CallFunction|SaveRooms (.SavedRooms (Utilities|Struct|BreakS_SavedLevel (Utilities|Array|Get(acopy) _savedlevels _output_get))))
  (CallFunction|SaveDungeons (.SavedDungeons (Utilities|Struct|BreakS_SavedLevel (Utilities|Array|Get(acopy) _savedlevels _output_get))))
  (CallFunction|SaveActors (.SavedActors (Utilities|Struct|BreakS_SavedLevel (Utilities|Array|Get(acopy) _savedlevels _output_get))))
  (CallFunction|SavePlayer _savedlevels _output_get)
  (SaveGame|SaveGametoSlot (Variables|Default|GetSavegames) SlotName))

(event Custom|LoadLevel
  (params (SlotName :type String))
  (bind _savegames (Variables|Default|GetSavegames))
  ;[1 1 1] Load
  (Variables|/Game/DungeonGenerator/Savegames/BP_Savegame.BP_Savegame_C|SetSlotToLoad _savegames SlotName)
  (SaveGame|SaveGametoSlot _savegames "LoadLevel")
  (bind _returnvalue (SaveGame|LoadGamefromSlot SlotName))
  (bind _asbp_savegame (Utilities|Casting|CastToBP_Savegame _returnvalue))
  (Game|OpenLevel(byName) (Utilities|String|StringToName (Variables|/Game/DungeonGenerator/Savegames/BP_Savegame.BP_Savegame_C|GetCurrentLevel _asbp_savegame))))

(event EventBeginPlay
  ;[1 1 1] Begin Play
  (Utilities|FlowControl|Sequence
    (:then_0
      ;[1 1 1] Load profile
      (bind _returnvalue (SaveGame|CreateSaveGameObject "/Game/DungeonGenerator/Savegames/BP_Profiles.BP_Profiles_C"))
      (Variables|Default|SetProfiles _returnvalue)
      (bind _returnvalue_2 (SaveGame|LoadGamefromSlot "CurrentProfile"))
      (bind _asbp_profiles (Utilities|Casting|CastToBP_Profiles _returnvalue_2))
      (Variables|Default|SetProfileName (Variables|/Game/DungeonGenerator/Savegames/BP_Profiles.BP_Profiles_C|GetProfileName _asbp_profiles)))
    (:then_1
      ;[1 1 1] UI
      (bind _returnvalue_3 (UserInterface|CreateWidget "/Game/DungeonGenerator/UI/UI_Menu.UI_Menu_C"))
      (Variables|Default|SetUI_Menu _returnvalue_3)
      (bind _returnvalue_4 (SaveGame|CreateSaveGameObject "/Game/DungeonGenerator/Savegames/BP_Savegame.BP_Savegame_C"))
      (Variables|Default|SetSavegames _returnvalue_4))
    (:then_2
      ;[1 1 1] If level was opened by loading game then load game
      (bind _returnvalue_5 (SaveGame|LoadGamefromSlot "LoadLevel"))
      (bind _asbp_savegame (Utilities|Casting|CastToBP_Savegame _returnvalue_5))
      (if (not (Utilities|Enum|Equal(Enum) (Variables|/Game/DungeonGenerator/Savegames/BP_Savegame.BP_Savegame_C|GetSlotToLoad _asbp_savegame) "None"))
        (Utilities|FlowControl|Delay 0.0)
        (CallFunction|LoadGame (Variables|/Game/DungeonGenerator/Savegames/BP_Savegame.BP_Savegame_C|GetSlotToLoad _asbp_savegame))))))

(fn LoadPlayer
  (params (S_SaveMainCharacter :type S%20Save%20Main%20Character%20Structure%20%28by%20ref%29))
  (bind (_location _rotation _maps _keys) (Utilities|Struct|BreakS_SaveMainCharacter S_SaveMainCharacter))
  (bind _returnvalue (Game|GetPlayerCharacter 0))
  (Transformation|SetActorLocationAndRotation _returnvalue _location _rotation)
  (Variables|/Game/DungeonGenerator/Blueprints/BP_MapComponent.BP_MapComponent_C|SetMaps (Actor|GetComponentbyClass _returnvalue "/Game/DungeonGenerator/Blueprints/BP_MapComponent.BP_MapComponent_C") _maps)
  (Variables|/Game/DungeonGenerator/Blueprints/BP_KeyRing.BP_KeyRing_C|SetKeys (Actor|GetComponentbyClass _returnvalue "/Game/DungeonGenerator/Blueprints/BP_KeyRing.BP_KeyRing_C") _keys)
  (return))

(fn LoadActors
  (params (SavedActors :type Array%20of%20S%20Saved%20Actors%20Structures))
  (for _array_element (Variables|Default|GetActorsToSave)
    (bind _outactors (Actor|GetAllActorsOfClass _array_element))
    (for _array_element_2 _outactors
      (if (and (!= (Actor|GetParentActor _array_element_2) "/Game/DungeonGenerator/Blueprints/BP_DungeonRoom.BP_DungeonRoom") (!= (Actor|GetParentActor _array_element_2) "/Game/DungeonGenerator/Blueprints/BP_DungeonGenerator.BP_DungeonGenerator"))
        (LocalVariables|SetLocalActorFound false)
        (for _array_element_3 SavedActors
          (if (== _array_element_2 (.ActorObject (Utilities|Struct|BreakS_SavedActors _array_element_3)))
            (LocalVariables|SetLocalActorFound true)))
        (if (not (LocalVariables|GetLocalActorFound))
          (Actor|DestroyActor _array_element_2)))))
  (for _array_element_4 SavedActors
    (Utilities|IsValid (.ActorObject (Utilities|Struct|BreakS_SavedActors _array_element_4))
      (:Is%20Valid
        (Transformation|SetActorLocationAndRotation (.ActorObject (Utilities|Struct|BreakS_SavedActors _array_element_4)) (.Location (Utilities|Struct|BreakS_SavedActors _array_element_4)) (.Rotation (Utilities|Struct|BreakS_SavedActors _array_element_4))))
      (:Is%20Not%20Valid
        (Game|SpawnActorfromClass (.ActorClass (Utilities|Struct|BreakS_SavedActors _array_element_4)) (Math|Transform|MakeTransform (.Location (Utilities|Struct|BreakS_SavedActors _array_element_4)) (.Rotation (Utilities|Struct|BreakS_SavedActors _array_element_4)) "1.000000,1.000000,1.000000") "Undefined" 0 0))))
  (return))

(fn LoadDungeon
  (params (Array :type Array%20of%20S%20Saved%20Dungeon%20Structures))
  (for _array_element Array
    (bind _asbp_dungeon_generator (Utilities|Casting|CastToBP_DungeonGenerator (.ActorObject (Utilities|Struct|BreakS_SavedDungeon _array_element))))
    (Default|LoadDungeon _asbp_dungeon_generator (.SavedDungeonRooms (Utilities|Struct|BreakS_SavedDungeon _array_element))))
  (return))

(fn LoadRooms
  (params (Array :type Array%20of%20S%20Saved%20Room%20Structures))
  (for _array_element Array
    (bind _asbp_dungeon_room (Utilities|Casting|CastToBP_DungeonRoom (.ActorObject (Utilities|Struct|BreakS_SavedRoom _array_element))))
    (Default|LoadRoom _asbp_dungeon_room (.SavedActors (Utilities|Struct|BreakS_SavedRoom _array_element)) (.SavedSpawenedActors (Utilities|Struct|BreakS_SavedRoom _array_element)) (.SavedAssets (Utilities|Struct|BreakS_SavedRoom _array_element)) (.Doors (Utilities|Struct|BreakS_SavedRoom _array_element))))
  (return))

(fn SaveRooms
  (params (TargetArray :type Array%20of%20S%20Saved%20Room%20Structures))
  (bind _outactors (Actor|GetAllActorsOfClass "/Game/DungeonGenerator/Blueprints/BP_DungeonRoom.BP_DungeonRoom_C"))
  (for _array_element _outactors
    (Utilities|Casting|CastToBP_DungeonGenerator (Actor|GetParentActor _array_element)
      (:CastFailed
        (bind _output_get (Default|SaveRoom _array_element))
        (Utilities|Array|Add TargetArray _output_get))))
  (return))

(fn SaveDungeons
  (params (TargetArray :type Array%20of%20S%20Saved%20Dungeon%20Structures))
  (bind _outactors (Actor|GetAllActorsOfClass "/Game/DungeonGenerator/Blueprints/BP_DungeonGenerator.BP_DungeonGenerator_C"))
  (for _array_element _outactors
    (bind _saveddungeon (Default|SaveDungeon _array_element))
    (Utilities|Array|Add TargetArray (Utilities|Struct|MakeS_SavedDungeon _array_element _saveddungeon)))
  (return))

(fn SaveActors
  (params (TargetArray :type Array%20of%20S%20Saved%20Actors%20Structures))
  (for _array_element (Variables|Default|GetActorsToSave)
    (bind _outactors (Actor|GetAllActorsOfClass _array_element))
    (for _array_element_2 _outactors
      (if (and (!= (Actor|GetParentActor _array_element_2) "/Game/DungeonGenerator/Blueprints/BP_DungeonRoom.BP_DungeonRoom") (!= (Actor|GetParentActor _array_element_2) "/Game/DungeonGenerator/Blueprints/BP_DungeonGenerator.BP_DungeonGenerator"))
        (Utilities|Array|Add TargetArray (Utilities|Struct|MakeS_SavedActors _array_element_2 (Utilities|GetClass _array_element_2) (Transformation|GetActorLocation _array_element_2) (Transformation|GetActorRotation _array_element_2))))))
  (return))

(fn SavePlayer
  (params (S_SavedLevels :type Array%20of%20S%20Saved%20Level%20Structures) (Index :type Integer))
  (bind _returnvalue (Game|GetPlayerCharacter 0))
  (bind _output (Utilities|Array|Get(acopy) S_SavedLevels Index))
  (bind (_levelname _savedrooms _saveddungeons _savedactors) (Utilities|Struct|BreakS_SavedLevel _output))
  (Utilities|Array|SetArrayElem S_SavedLevels Index (Utilities|Struct|MakeS_SavedLevel _levelname _savedrooms _saveddungeons _savedactors (Utilities|Struct|MakeS_SaveMainCharacter (Transformation|GetActorLocation _returnvalue) (Transformation|GetActorRotation _returnvalue) (Variables|/Game/DungeonGenerator/Blueprints/BP_MapComponent.BP_MapComponent_C|GetMaps (Actor|GetComponentbyClass _returnvalue "/Game/DungeonGenerator/Blueprints/BP_MapComponent.BP_MapComponent_C")) (Variables|/Game/DungeonGenerator/Blueprints/BP_KeyRing.BP_KeyRing_C|GetKeys (Actor|GetComponentbyClass _returnvalue "/Game/DungeonGenerator/Blueprints/BP_KeyRing.BP_KeyRing_C")))))
  (return))

(fn SaveLevel
  (bind _savegames (Variables|Default|GetSavegames))
  (bind _savedlevels (Variables|/Game/DungeonGenerator/Savegames/BP_Savegame.BP_Savegame_C|GetSavedLevels _savegames))
  (bind _returnvalue (Game|GetCurrentLevelName true))
  (Variables|/Game/DungeonGenerator/Savegames/BP_Savegame.BP_Savegame_C|SetCurrentLevel _savegames _returnvalue)
  (LocalVariables|SetLocalLevelFound false)
  (bind (_array_element _array_index) (Utilities|Array|ForEachLoopwithBreak _savedlevels :!label _label)
    (:LoopBody
      (bind _returnvalue_2 (Game|GetCurrentLevelName true))
      (if (Utilities|Enum|Equal(Enum) _returnvalue_2 (.LevelName (Utilities|Struct|BreakS_SavedLevel _array_element)))
        (LocalVariables|SetLocalLevelFound true)
        (Utilities|FlowControl|Sequence
          (:then_0
            (goto _label Break))
          (:then_1
            (return _array_index)))))
    (:Completed
      (if (not (LocalVariables|GetLocalLevelFound))
        (bind _returnvalue_3 (Game|GetCurrentLevelName true))
        (bind _returnvalue_4 (Utilities|Array|Add _savedlevels (Utilities|Struct|MakeS_SavedLevel _returnvalue_3 (Utilities|Array|MakeArray "") (Utilities|Array|MakeArray "") (Utilities|Array|MakeArray ""))))
        (return _returnvalue_4)))))