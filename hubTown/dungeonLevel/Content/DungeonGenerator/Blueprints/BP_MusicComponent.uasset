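; Music component that plays one 2D sound at a time, crossfading when Play receives a different track.
; Each new track fades in while the previous one is unbound and faded out.
; When audio finishes, the track restarts from zero, giving a manual loop.
; Pause stops the audio, and Unpause recreates it using Timer, a variable written on Tick, as the start time.
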(event Custom|Play
  (params (Sound :type Sound%20Cue%20Object%20Reference))
  ;[1 1 1] Play / Pause
  (if (not (== Sound (Variables|Default|GetSound)))
    (Variables|Default|SetSound Sound)
    (Variables|Default|SetTimer 0.0)
    (Utilities|IsValid (Variables|Default|GetTunePlaying)
      (:Is%20Valid
        (EventDispatchers|UnbindallEventsfromOnAudioFinished (Variables|Default|GetTunePlaying))
        (Audio|Components|Audio|FadeOut (Variables|Default|GetTunePlaying) (Variables|Default|GetFade) 0.0 "Linear" :!class /Script/Engine.AudioComponent))
      (:Is%20Not%20Valid
        _))
    (bind _returnvalue (Audio|CreateSound2D (Variables|Default|GetSound) 1.0 1.0 (Variables|Default|GetTimer) 0))
    (bind _output_get (Variables|Default|SetTunePlaying _returnvalue))
    (Audio|Components|Audio|FadeIn _output_get (Variables|Default|GetFade) 1.0 (Variables|Default|GetTimer) "Linear" :!class /Script/Engine.AudioComponent)
    (EventDispatchers|AssignOnAudioFinished _returnvalue (delegate Custom|OnAudioFinished_Event_0))))

(event Custom|Pause
  ;[1 1 1] Play / Pause
  (Audio|Components|Audio|Stop (Variables|Default|GetTunePlaying)))

(event Custom|Unpause
  ;[1 1 1] Play / Pause
  (bind _returnvalue (Audio|CreateSound2D (Variables|Default|GetSound) 1.0 1.0 (Variables|Default|GetTimer) 0))
  (bind _output_get (Variables|Default|SetTunePlaying _returnvalue))
  (Audio|Components|Audio|FadeIn _output_get (Variables|Default|GetFade) 1.0 (Variables|Default|GetTimer) "Linear" :!class /Script/Engine.AudioComponent)
  (EventDispatchers|AssignOnAudioFinished _returnvalue (delegate Custom|OnAudioFinished_Event_0)))

(event Custom|OnAudioFinished_Event_0
  ;[1 1 1] Play / Pause
  (Variables|Default|SetTimer 0.0)
  (bind _returnvalue (Audio|CreateSound2D (Variables|Default|GetSound) 1.0 1.0 (Variables|Default|GetTimer) 0))
  (bind _output_get (Variables|Default|SetTunePlaying _returnvalue))
  (Audio|Components|Audio|FadeIn _output_get (Variables|Default|GetFade) 1.0 (Variables|Default|GetTimer) "Linear" :!class /Script/Engine.AudioComponent)
  (EventDispatchers|AssignOnAudioFinished _returnvalue (delegate Custom|OnAudioFinished_Event_0)))

(event EventTick
  (params (DeltaSeconds :type Float%20%28single-precision%29))
  ;[1 1 1] Timer
  (Variables|Default|SetTimer DeltaSeconds))