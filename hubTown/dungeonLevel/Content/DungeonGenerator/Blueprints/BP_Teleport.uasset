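; Teleporter for the dungeon generator that moves overlapping actors, or only the player, to a dungeon entrance, linked teleport, target point or fixed location.
; Dungeon entrance spots derive from entrance direction, tile size and grid size.
; BeginPlay can spawn a linked return teleport, and construction back-links paired teleports and selects 2D or 3D visuals.
; An ActorsEntered list on each teleport keeps linked pairs from bouncing actors straight back.
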(event EventBeginPlay
  (bind _self self)
  (bind _backway_teleport (Variables|Default|GetBackway_Teleport))
  (bind _backway_teleport_2 (Variables|Default|GetBackway_Teleport))
  (bind _backway_teleport_3 (Variables|Default|GetBackway_Teleport))
  (bind _totargetpoint (Variables|Default|GetToTargetPoint))
  (bind _returnvalue (Utilities|GetClass _self))
  ;[1 1 1] BeginPlay, Spawn Backway Teleports
  (if (and (Variables|Default|GetCreateBackwayTeleport) (not (Utilities|IsValid (Variables|Default|GetToTeleport))))
    (Utilities|IsValid (Variables|Default|GetToDungeon)
      (:Is%20Valid
        (bind (_locationto _rotarion _locationbackway) (CallFunction|DungeonEntranceLocation (Variables|Default|GetToDungeon)))
        (bind _returnvalue_2 (Game|SpawnActorfromClass _returnvalue (Math|Transform|MakeTransform _locationbackway _rotarion "1,1,1") "Undefined" 0 (Variables|Default|GetVisible) 0))
        (Variables|Default|SetToTeleport _returnvalue_2)
        (Utilities|IsValid _backway_teleport_2
          (:Is%20Valid
            (Variables|BP_Teleport_C|SetToTeleport _returnvalue_2 _backway_teleport_2))
          (:Is%20Not%20Valid
            (Variables|BP_Teleport_C|SetToTeleport _returnvalue_2 self))))
      (:Is%20Not%20Valid
        (Utilities|IsValid (Variables|Default|GetToTargetPoint)
          (:Is%20Valid
            (bind _returnvalue_3 (Game|SpawnActorfromClass _returnvalue (Math|Transform|MakeTransform (Transformation|GetActorLocation _totargetpoint) (Transformation|GetActorRotation _totargetpoint) "1,1,1") "Undefined" 0 (Variables|Default|GetVisible) 0))
            (Variables|Default|SetToTeleport _returnvalue_3)
            (Utilities|IsValid _backway_teleport_3
              (:Is%20Valid
                (Variables|BP_Teleport_C|SetToTeleport _returnvalue_3 _backway_teleport_3))
              (:Is%20Not%20Valid
                (Variables|BP_Teleport_C|SetToTeleport _returnvalue_3 self))))
          (:Is%20Not%20Valid
            (bind _returnvalue_4 (Game|SpawnActorfromClass _returnvalue (Math|Transform|MakeTransform (Variables|Default|GetToLocation) "0, 0, 0" "1,1,1") "Undefined" 0 (Variables|Default|GetVisible) 0))
            (Variables|Default|SetToTeleport _returnvalue_4)
            (Utilities|IsValid _backway_teleport
              (:Is%20Valid
                (Variables|BP_Teleport_C|SetToTeleport _returnvalue_4 _backway_teleport))
              (:Is%20Not%20Valid
                (Variables|BP_Teleport_C|SetToTeleport _returnvalue_4 self)))))))))

(event Collision|EventActorBeginOverlap
  (params (OtherActor :type Actor%20Object%20Reference))
  (bind _toteleport (Variables|Default|GetToTeleport))
  (bind _totargetpoint (Variables|Default|GetToTargetPoint))
  ;[1 1 1] Entering teleport
  (if (Variables|Default|GetOnlyPlayers)
    (if (== OtherActor (Game|GetPlayerCharacter 0))
      (if (not (Utilities|Array|ContainsItem (Variables|Default|GetActors_Entered) OtherActor)) :!label _label
        (bind _output_get (Variables|Default|SetActor OtherActor))
        (Utilities|Array|Add (Variables|Default|GetActors_Entered) _output_get)
        (Utilities|IsValid (Variables|Default|GetToDungeon)
          (:Is%20Valid
            (bind (_locationto _rotarion) (CallFunction|DungeonEntranceLocation (Variables|Default|GetToDungeon)))
            (CallFunction|TeleportCustom (Variables|Default|GetActor) _locationto _rotarion))
          (:Is%20Not%20Valid
            (Utilities|IsValid (Variables|Default|GetToTeleport)
              (:Is%20Valid
                (Utilities|Array|AddUnique (Variables|BP_Teleport_C|GetActors_Entered _toteleport) (Variables|Default|GetActor))
                (CallFunction|TeleportCustom (Variables|Default|GetActor) (Transformation|GetActorLocation _toteleport) (Transformation|GetActorRotation _toteleport)))
              (:Is%20Not%20Valid
                (Utilities|IsValid (Variables|Default|GetToTargetPoint)
                  (:Is%20Valid
                    (CallFunction|TeleportCustom 0 (Transformation|GetActorLocation _totargetpoint) (Transformation|GetActorRotation _totargetpoint)))
                  (:Is%20Not%20Valid
                    (CallFunction|TeleportCustom 0 (Variables|Default|GetToLocation) "0, 0, 0")))))))))
    (else
      (goto _label))))

(event Collision|EventActorEndOverlap
  (params (OtherActor :type Actor%20Object%20Reference))
  ;[1 1 1] Leaving teleport
  (Utilities|IsValid (Variables|Default|GetToTeleport)
    (:Is%20Valid
      (if (Variables|Default|GetOnlyPlayers)
        (if (== OtherActor (Game|GetPlayerCharacter 0))
          (Utilities|Array|RemoveItem (Variables|Default|GetActors_Entered) OtherActor :!label _label))
        (else
          (goto _label))))))

(fn ConstructionScript
  (Utilities|FlowControl|Sequence
    (:then_0
      ;[1 1 1] Seting teleport link in another teleport
      (Utilities|IsValid (Variables|Default|GetToTeleport)
        (:Is%20Valid
          (Utilities|IsValid (Variables|BP_Teleport_C|GetToTeleport (Variables|Default|GetToTeleport))
            (:Is%20Not%20Valid
              (Variables|BP_Teleport_C|SetToTeleport (Variables|Default|GetToTeleport) self))))))
    (:then_1
      ;[1 1 1] 2D/3D
      (if (Variables|Default|Get3D)
        (CallFunction|RemoveSceneAssets (Variables|Default|GetScene_2D))
        (else
          (CallFunction|RemoveSceneAssets (Variables|Default|GetScene_3D)))))
    (:then_2
      (Rendering|SetVisibility (Variables|Default|GetScene_Visuals) (Variables|Default|GetVisible) true))))

(fn TeleportCustom
  (params (Actor :type Actor%20Object%20Reference) (Location :type Vector) (DestRotation :type Rotator))
  (if (Variables|Default|Get3D)
    (LocalVariables|SetLocalTeleportzOffset (Variables|Default|GetTeleport_zOffset_3D))
    (else
      (LocalVariables|SetLocalTeleportzOffset (Variables|Default|GetTeleport_zOffset_2D))))
  (Transformation|Teleport Actor (Math|Vector|MakeVector (.x Location) (.y Location) (+ (.z Location) (LocalVariables|GetLocalTeleportzOffset))) DestRotation))

(fn DungeonEntranceLocation
  (params (Dungeon :type BP%20Dungeon%20Generator%20Object%20Reference))
  (bind _returnvalue (Transformation|GetActorLocation Dungeon))
  (bind _tilesize (Variables|/Game/DungeonGenerator/Blueprints/BP_DungeonGenerator.BP_DungeonGenerator_C|GetTileSize Dungeon))
  (bind _tilesxy (Variables|/Game/DungeonGenerator/Blueprints/BP_DungeonGenerator.BP_DungeonGenerator_C|GetTilesXY Dungeon))
  (bind _tilesscale (Variables|/Game/DungeonGenerator/Blueprints/BP_DungeonGenerator.BP_DungeonGenerator_C|GetTilesScale Dungeon))
  (bind _returnvalue_2 (/ _tilesxy 2.0))
  (bind _returnvalue_3 (* _tilesize _tilesscale))
  (bind _returnvalue_4 (- _returnvalue_2 0.5))
  (bind _returnvalue_5 (- _returnvalue_2 1.5))
  (bind _returnvalue_6 (* _returnvalue_3 _returnvalue_4))
  (bind _returnvalue_7 (* _returnvalue_3 _returnvalue_5))
  (bind (_x _y) (Math|Vector2D|BreakVector2D _returnvalue_6))
  (bind (_x_2 _y_2) (Math|Vector2D|BreakVector2D _returnvalue_7))
  (switch Utilities|FlowControl|Switch|SwitchonE_RoomsDoors (Variables|/Game/DungeonGenerator/Blueprints/BP_DungeonGenerator.BP_DungeonGenerator_C|GetFirstRoomEntranceDirection Dungeon)
    (:NewEnumerator0
      (LocalVariables|SetLocalLocation (Math|Vector|MakeVector (+ (.x _returnvalue) _x_2) (.y _returnvalue) (.z _returnvalue)))
      (LocalVariables|SetLocalRotation "0,180.000000, 0")
      (LocalVariables|SetLocalLocationBackway (Math|Vector|MakeVector (+ (.x _returnvalue) _x) (.y _returnvalue) (.z _returnvalue))))
    (:NewEnumerator1
      (LocalVariables|SetLocalLocation (Math|Vector|MakeVector (- (.x _returnvalue) _x_2) (.y _returnvalue) (.z _returnvalue)))
      (LocalVariables|SetLocalRotation "0, 0, 0")
      (LocalVariables|SetLocalLocationBackway (Math|Vector|MakeVector (- (.x _returnvalue) _x) (.y _returnvalue) (.z _returnvalue))))
    (:NewEnumerator2
      (LocalVariables|SetLocalLocation (Math|Vector|MakeVector (.x _returnvalue) (- (.y _returnvalue) _y_2) (.z _returnvalue)))
      (LocalVariables|SetLocalRotation "0,90.000000, 0")
      (LocalVariables|SetLocalLocationBackway (Math|Vector|MakeVector (.x _returnvalue) (- (.y _returnvalue) _y) (.z _returnvalue))))
    (:NewEnumerator3
      (LocalVariables|SetLocalLocation (Math|Vector|MakeVector (.x _returnvalue) (+ _y_2 (.y _returnvalue)) (.z _returnvalue)))
      (LocalVariables|SetLocalRotation "0,-90.000000, 0")
      (LocalVariables|SetLocalLocationBackway (Math|Vector|MakeVector (.x _returnvalue) (+ (.y _returnvalue) _y) (.z _returnvalue)))))
  (return (LocalVariables|GetLocalLocation) (LocalVariables|GetLocalRotation) (LocalVariables|GetLocalLocationBackway)))