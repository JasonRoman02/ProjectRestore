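; BP_Key is a key pickup actor in the dungeon generator.
; When an overlapping actor has a BP_KeyRing component, it adds its KeyName to that component's Keys once, plays an optional pickup sound and destroys itself.
; The construction script uses the 3D flag to remove the assets of the unused scene, keeping either the 2D or 3D representation.
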(event Collision|EventActorBeginOverlap
  (params (OtherActor :type Actor%20Object%20Reference))
  (bind _returnvalue (Actor|GetComponentbyClass OtherActor "/Game/DungeonGenerator/Blueprints/BP_KeyRing.BP_KeyRing_C"))
  (bind _sfx_pickupkey (Variables|Default|GetSFX_PickupKey))
  (|CallParentFunction OtherActor)
  (Utilities|IsValid _returnvalue
    (:Is%20Valid
      (Utilities|FlowControl|DoOnce false
        (:Completed
          (Utilities|Array|Add (Variables|/Game/DungeonGenerator/Blueprints/BP_KeyRing.BP_KeyRing_C|GetKeys _returnvalue) (Variables|Default|GetKeyName))
          (Utilities|IsValid _sfx_pickupkey
            (:Is%20Valid
              (Audio|PlaySoundatLocation _sfx_pickupkey (Transformation|GetActorLocation) "0, 0, 0" 1.0 1.0 0.0 0 0 0))
            (:Is%20Not%20Valid
              _))
          (Actor|DestroyActor))))))

(fn ConstructionScript
  (|CallParentFunction)
  (if (Variables|Default|Get3D)
    (CallFunction|RemoveSceneAssets (Variables|Default|GetScene_2D))
    (else
      (CallFunction|RemoveSceneAssets (Variables|Default|GetScene_3D)))))