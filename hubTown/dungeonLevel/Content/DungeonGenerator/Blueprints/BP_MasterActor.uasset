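; BP_MasterActor is a dungeon generator actor that provides shared setup and cleanup logic, with no active event logic.
; Its construction script copies the 3D variable from its parent actor when that parent is also a BP_MasterActor, so nested child actors inherit the setting.
; RemoveSceneAssets gathers all descendants of a given scene component into a local list, destroys them, then destroys the component itself.
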(event EventBeginPlay)

(event Collision|EventActorBeginOverlap
  (params (OtherActor :type Actor%20Object%20Reference)))

(event EventTick
  (params (DeltaSeconds :type Float%20%28single-precision%29)))

(fn ConstructionScript
  (bind _asbp_master_actor (Utilities|Casting|CastToBP_MasterActor (Actor|GetParentActor)))
  (Variables|Default|Set3D (Variables|BP_MasterActor_C|Get3D _asbp_master_actor)))

(fn RemoveSceneAssets
  (params (SceneComponent :type Scene%20Component%20Object%20Reference))
  (for _array_element (Components|GetChildrenComponents SceneComponent true)
    (Utilities|Array|Add (LocalVariables|GetLocalSceneComponents) _array_element))
  (for _array_element_2 (LocalVariables|GetLocalSceneComponents)
    (Components|DestroyComponent _array_element_2))
  (Components|DestroyComponent SceneComponent)
  (return))