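; BP_Map is a map pickup for the dungeon generator that reveals the whole map when collected.
; On overlap with an actor that has a BP_MapComponent, it calls FullMapReveal once, plays an optional pickup sound and destroys itself.
; The construction script uses the 3D flag to keep either the 2D or 3D scene assets and remove the other set.
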(event Collision|EventActorBeginOverlap
  (params (OtherActor :type Actor%20Object%20Reference))
  (bind _returnvalue (Actor|GetComponentbyClass OtherActor "/Game/DungeonGenerator/Blueprints/BP_MapComponent.BP_MapComponent_C"))
  (bind _sfx_pickupmap (Variables|Default|GetSFX_PickupMap))
  (|CallParentFunction OtherActor)
  (Utilities|IsValid _returnvalue
    (:Is%20Valid
      (Utilities|FlowControl|DoOnce false
        (:Completed
          (Default|FullMapReveal _returnvalue)
          (Utilities|IsValid _sfx_pickupmap
            (:Is%20Valid
              (Audio|PlaySoundatLocation _sfx_pickupmap (Transformation|GetActorLocation) "0, 0, 0" 1.0 1.0 0.0 0 0 0))
            (:Is%20Not%20Valid
              _))
          (Actor|DestroyActor))))))

(fn ConstructionScript
  (|CallParentFunction)
  (if (Variables|Default|Get3D)
    (CallFunction|RemoveSceneAssets (Variables|Default|GetScene_2D))
    (else
      (CallFunction|RemoveSceneAssets (Variables|Default|GetScene_3D)))))