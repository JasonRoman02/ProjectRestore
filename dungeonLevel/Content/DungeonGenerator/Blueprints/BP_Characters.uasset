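; Dungeon generator character actor that supports both 2D and 3D visual versions, with placeholder behavior for demonstrating door functionality.
; After the parent construction script runs, the 3D flag decides whether the Scene2D or Scene3D assets are removed.
; At runtime the actor destroys itself when the player character overlaps its sphere, a demo stand-in for custom logic.
; NewFunction_0 destroys all Scene2D child components but is not called in this graph.
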(event OnComponentBeginOverlap(Sphere)
  (params (OverlappedComponent :type Primitive%20Component%20Object%20Reference) (OtherActor :type Actor%20Object%20Reference) (OtherComp :type Primitive%20Component%20Object%20Reference) (OtherBodyIndex :type Integer) (bFromSweep :type Boolean) (SweepResult :type Hit%20Result%20Structure%20%28by%20ref%29))
  ;[1 1 1] Self destruct when player gets close (for demonstration doors functionality, to be deleted and replaced with custom logic)
  (if (== OtherActor (Game|GetPlayerCharacter 0))
    (Actor|DestroyActor)))

(event EventBeginPlay)

(event Collision|EventActorBeginOverlap
  (params (OtherActor :type Actor%20Object%20Reference)))

(event EventTick
  (params (DeltaSeconds :type Float%20%28single-precision%29)))

(fn ConstructionScript
  (|CallParentFunction)
  (if (Variables|Default|Get3D)
    (CallFunction|RemoveSceneAssets (Variables|Default|GetScene_2D))
    (else
      (CallFunction|RemoveSceneAssets (Variables|Default|GetScene_3D)))))

(fn NewFunction0
  (for _array_element (Components|GetChildrenComponents (Variables|Default|GetScene_2D) true)
    (Components|DestroyComponent _array_element)))