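; Configurable dungeon door that works as a 2D Paper2D or 3D single or double door, unlocked by a matching key.
; The construction script destroys unused variant components and applies the initial open state.
; Box overlap consumes the key from the actor's BP_KeyRing, then opens the door.
; 3D leaves slide via MoveComponentTo, while 2D plays a temporary flipbook, reversed for closing, then swaps sprite and collision.
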(event OnComponentBeginOverlap(Box)
  (params (OverlappedComponent :type Primitive%20Component%20Object%20Reference) (OtherActor :type Actor%20Object%20Reference) (OtherComp :type Primitive%20Component%20Object%20Reference) (OtherBodyIndex :type Integer) (bFromSweep :type Boolean) (SweepResult :type Hit%20Result%20Structure%20%28by%20ref%29))
  (bind _returnvalue (Actor|GetComponentbyClass OtherActor "/Game/DungeonGenerator/Blueprints/BP_KeyRing.BP_KeyRing_C"))
  (bind _sfx_unlock (Variables|Default|GetSFX_Unlock))
  (bind _keys (Variables|/Game/DungeonGenerator/Blueprints/BP_KeyRing.BP_KeyRing_C|GetKeys _returnvalue))
  ;[1 1 1] Unlock
  (if (Utilities|Name|NotEqual(Name) (Variables|Default|GetKey) "None")
    (if (not (Variables|Default|GetOpened))
      (bind (_array_element _array_index) (Utilities|Array|ForEachLoopwithBreak _keys :!label _label)
        (:LoopBody
          (if (Utilities|Name|Equal(Name) _array_element (Variables|Default|GetKey))
            (Utilities|FlowControl|Sequence
              (:then_0
                (goto _label Break))
              (:then_1
                (Utilities|Array|RemoveIndex _keys _array_index)
                (CallFunction|Open)
                (Utilities|IsValid _sfx_unlock
                  (:Is%20Valid
                    (Audio|PlaySoundatLocation _sfx_unlock (Transformation|GetActorLocation) "0, 0, 0" 1.0 1.0 0.0 0 0 0 0)))))))))))

(event Custom|CloseDoubleDoor_3D
  (bind _overtime (Variables|Default|GetOverTime))
  ;[1 1 1] OpenClose
  ;;[1 1 1] 3D
  ;;;[1 1 1] DoubleDoor
  (if (Variables|Default|GetOpened)
    (Variables|Default|SetOpened false)
    (Utilities|FlowControl|Sequence
      (:then_0
        (Components|MoveComponentTo (Variables|Default|GetScene_DoubleDoor_L) (Variables|Default|GetDoor_LR_OpenPosition_3D) "0, 0, 0" true true (Variables|Default|GetOverTime) false) ; enters at Stop
      )
      (:then_1
        (Components|MoveComponentTo (Variables|Default|GetScene_DoubleDoor_L) "0, 0, 0" "0, 0, 0" true true _overtime false))
      (:then_2
        (Components|MoveComponentTo (Variables|Default|GetScene_DoubleDoor_R) "0, 0, 0" "0, 0, 0" true true _overtime false)))))

(event Custom|OpenDoubleDoor_3D
  (bind _door_lr_openposition_3d (Variables|Default|GetDoor_LR_OpenPosition_3D))
  (bind _overtime (Variables|Default|GetOverTime))
  ;[1 1 1] OpenClose
  ;;[1 1 1] 3D
  ;;;[1 1 1] DoubleDoor
  (if (not (Variables|Default|GetOpened))
    (Variables|Default|SetOpened true)
    (Utilities|FlowControl|Sequence
      (:then_0
        (Components|MoveComponentTo (Variables|Default|GetScene_DoubleDoor_L) "0, 0, 0" "0, 0, 0" true true (Variables|Default|GetOverTime) false) ; enters at Stop
      )
      (:then_1
        (Components|MoveComponentTo (Variables|Default|GetScene_DoubleDoor_L) _door_lr_openposition_3d "0, 0, 0" true true _overtime false))
      (:then_2
        (Components|MoveComponentTo (Variables|Default|GetScene_DoubleDoor_R) (* _door_lr_openposition_3d -1.0) "0, 0, 0" true true _overtime false)))))

(event Custom|Close_2D
  (bind _papersprite (Variables|Default|GetPaperSprite))
  ;[1 1 1] OpenClose
  ;;[1 1 1] 2D
  (if (Variables|Default|GetOpened)
    (Variables|Default|SetOpened false)
    (Rendering|SetVisibility _papersprite false false)
    (bind _returnvalue (AddComponent|AddPaperFlipbookComponent false (Transformation|GetRelativeTransform _papersprite)))
    (Transformation|AttachComponentToComponent _returnvalue (Variables|Default|GetScene_2D) "None" "KeepRelative" "KeepRelative" "KeepRelative" true)
    (Components|Timeline|SetLooping _returnvalue false)
    (Sprite|SetFlipbook _returnvalue (Variables|Default|GetFlipbook_Open))
    (Components|Timeline|ReversefromEnd _returnvalue)
    (EventDispatchers|AssignOnFinishedPlaying _returnvalue (delegate Custom|OnFinishedPlaying_Event_1))))

(event Custom|Open_2D
  (bind _papersprite (Variables|Default|GetPaperSprite))
  ;[1 1 1] OpenClose
  ;;[1 1 1] 2D
  (if (not (Variables|Default|GetOpened))
    (Variables|Default|SetOpened true)
    (Rendering|SetVisibility _papersprite false false)
    (bind _returnvalue (AddComponent|AddPaperFlipbookComponent false (Transformation|GetRelativeTransform _papersprite)))
    (Transformation|AttachComponentToComponent _returnvalue (Variables|Default|GetScene_2D) "None" "KeepRelative" "KeepRelative" "KeepRelative" true)
    (Components|Timeline|SetLooping _returnvalue false)
    (Sprite|SetFlipbook _returnvalue (Variables|Default|GetFlipbook_Open))
    (EventDispatchers|AssignOnFinishedPlaying _returnvalue (delegate Custom|OnFinishedPlaying_Event_0))))

(event Custom|OnFinishedPlaying_Event_0
  ;[1 1 1] OpenClose
  ;;[1 1 1] 2D
  (Components|DestroyComponent (stale Custom|Open_2D _returnvalue))
  (Rendering|Components|Sprite|SetSprite (Variables|Default|GetPaperSprite) (Variables|Default|GetSprite_Opened))
  (Rendering|SetVisibility (Variables|Default|GetPaperSprite) true false)
  (CallFunction|CollisionsonOff false (Variables|Default|GetScene_2D)))

(event Custom|OnFinishedPlaying_Event_1
  ;[1 1 1] OpenClose
  ;;[1 1 1] 2D
  (Components|DestroyComponent (stale Custom|Close_2D _returnvalue))
  (Rendering|Components|Sprite|SetSprite (Variables|Default|GetPaperSprite) (Variables|Default|GetSprite_Closed))
  (Rendering|SetVisibility (Variables|Default|GetPaperSprite) true false)
  (CallFunction|CollisionsonOff true (Variables|Default|GetScene_2D)))

(event Custom|OpenSingleDoor_3D
  ;[1 1 1] OpenClose
  ;;[1 1 1] 3D
  ;;;[1 1 1] SingleDoor
  (if (not (Variables|Default|GetOpened))
    (Variables|Default|SetOpened true)
    (Utilities|FlowControl|Sequence
      (:then_0
        (Components|MoveComponentTo (Variables|Default|GetScene_Door_Single) "0, 0, 0" "0, 0, 0" true true (Variables|Default|GetOverTime) false) ; enters at Stop
      )
      (:then_1
        (if (Variables|Default|Get3D)
          (Components|MoveComponentTo (Variables|Default|GetScene_Door_Single) (Variables|Default|GetSingleDoorOpenPosition_3D) "0, 0, 0" true true (Variables|Default|GetOverTime) false))))))

(event Custom|Close
  ;[1 1 1] OpenClose
  (if (Variables|Default|Get3D)
    (if (Variables|Default|GetDoubleDoor)
      (CallFunction|CloseDoubleDoor3D)
      (else
        (CallFunction|CloseSingleDoor3D)))
    (else
      (CallFunction|Close2D))))

(event Custom|Open
  ;[1 1 1] OpenClose
  (if (Variables|Default|Get3D)
    (if (Variables|Default|GetDoubleDoor)
      (CallFunction|OpenDoubleDoor3D)
      (else
        (CallFunction|OpenSingleDoor3D)))
    (else
      (CallFunction|Open2D))))

(event Custom|CloseSingleDoor_3D
  ;[1 1 1] OpenClose
  ;;[1 1 1] 3D
  ;;;[1 1 1] SingleDoor
  (if (Variables|Default|GetOpened)
    (Variables|Default|SetOpened false)
    (Utilities|FlowControl|Sequence
      (:then_0
        (Components|MoveComponentTo (Variables|Default|GetScene_Door_Single) (Variables|Default|GetSingleDoorOpenPosition_3D) "0, 0, 0" true true (Variables|Default|GetOverTime) false) ; enters at Stop
      )
      (:then_1
        (Components|MoveComponentTo (Variables|Default|GetScene_Door_Single) "0, 0, 0" "0, 0, 0" true true (Variables|Default|GetOverTime) false)))))

(event EventBeginPlay
  (for _array_element (Collision|GetOverlappingActors (Variables|Default|GetBox) "BP_Doors_C" :!class /Script/Engine.PrimitiveComponent)
    (bind _asbp_dungeon_room (Utilities|Casting|CastToBP_DungeonRoom _array_element))
    (if (Collision|IsOverlappingActor (Variables|Default|GetBox) _array_element :!class /Script/Engine.PrimitiveComponent)
      (Variables|Default|SetOpened true)
      (CallFunction|Open)
      (else
        (Variables|Default|SetLocked true)
        (CallFunction|Close)))))

(fn ConstructionScript
  (bind _door_lr_openposition_3d (Variables|Default|GetDoor_LR_OpenPosition_3D))
  (|CallParentFunction)
  (Utilities|FlowControl|Sequence
    (:then_0
      ;[1 1 1] 2D/3D
      (if (Variables|Default|Get3D)
        (CallFunction|RemoveSceneAssets (Variables|Default|GetScene_2D))
        ;[1 1 1] Double/Single
        (if (Variables|Default|GetDoubleDoor)
          (CallFunction|RemoveSceneAssets (Variables|Default|GetScene_Door_Single))
          (else
            (CallFunction|RemoveSceneAssets (Variables|Default|GetScene_DoubleDoor_L))
            (CallFunction|RemoveSceneAssets (Variables|Default|GetScene_DoubleDoor_R))))
        (else
          (CallFunction|RemoveSceneAssets (Variables|Default|GetScene_3D)))))
    (:then_1
      ;[1 1 1] Opened / Closed
      (if (Variables|Default|Get3D)
        ;;[1 1 1] 3D
        (if (Variables|Default|GetOpened)
          (Transformation|SetRelativeLocation (Variables|Default|GetScene_DoubleDoor_L) _door_lr_openposition_3d false false)
          (Transformation|SetRelativeLocation (Variables|Default|GetScene_DoubleDoor_R) (* _door_lr_openposition_3d -1) false false)
          (Transformation|SetRelativeLocation (Variables|Default|GetScene_Door_Single) (Variables|Default|GetSingleDoorOpenPosition_3D) false false)
          (else
            (Transformation|SetRelativeLocation (Variables|Default|GetScene_DoubleDoor_L) "0, 0, 0" false false)
            (Transformation|SetRelativeLocation (Variables|Default|GetScene_DoubleDoor_R) "0, 0, 0" false false)
            (Transformation|SetRelativeLocation (Variables|Default|GetScene_Door_Single) "0, 0, 0" false false)))
        (else
          ;;[1 1 1] 2D
          (if (Variables|Default|GetOpened)
            (Rendering|Components|Sprite|SetSprite (Variables|Default|GetPaperSprite) (Variables|Default|GetSprite_Opened))
            (CallFunction|CollisionsonOff false (Variables|Default|GetScene_2D))
            (else
              (Rendering|Components|Sprite|SetSprite (Variables|Default|GetPaperSprite) (Variables|Default|GetSprite_Closed))
              (CallFunction|CollisionsonOff true (Variables|Default|GetScene_2D)))))))))

(fn RemoveAssets
  (params (SceneComponent :type Scene%20Component%20Object%20Reference))
  (for _array_element (Components|GetChildrenComponents SceneComponent true)
    (Utilities|Array|Add (LocalVariables|GetLocalComponents) _array_element))
  (for _array_element_2 (LocalVariables|GetLocalComponents)
    (Components|DestroyComponent _array_element_2))
  (Components|DestroyComponent SceneComponent)
  (return))

(fn CollisionsonOff
  (params (On :type Boolean) (SceneComponent :type Scene%20Component%20Object%20Reference))
  (if On
    (LocalVariables|SetLocalCollisionSetting "QueryAndPhysics")
    (else
      (LocalVariables|SetLocalCollisionSetting "NoCollision")))
  (bind _output_get (LocalVariables|SetLocalChildComponents (Components|GetChildrenComponents SceneComponent true)))
  (if (> (Utilities|Array|Length _output_get) 0)
    (for _array_element _output_get
      (bind _aspaper_sprite_component (Utilities|Casting|CastToPaperSpriteComponent _array_element)
        (:then
          (Collision|SetCollisionEnabled _aspaper_sprite_component (LocalVariables|GetLocalCollisionSetting)))
        (:CastFailed
          (bind _aspaper_tile_map_component (Utilities|Casting|CastToPaperTileMapComponent _array_element))
          (Collision|SetCollisionEnabled _aspaper_tile_map_component (LocalVariables|GetLocalCollisionSetting))))))
  (return))